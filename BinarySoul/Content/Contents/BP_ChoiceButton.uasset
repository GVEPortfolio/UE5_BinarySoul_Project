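; BP_ChoiceButton is a choice button that displays a description and is built to send its ButtonData to the game instance.
; The construction script writes the description into the WBP_ButtonText of its widget component.
; A DoOnce, reset by BeginPlay and ResetButton, gates the ProcessChoice call on BP_GameInstance.
; OnInteracted and the gate's Enter sit in logic that never runs.
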(event `self.ReceiveBeginPlay`
  (`/Engine/EditorBlueprintResources/StandardMacros.DoOnce` false :!via `Reset` :!label _label
    (:`Completed`
      (bind _asbp_game_instance (cast `/Game/BP_GameInstance` (`GameplayStatics.GetGameInstance`)))
      (`BinaryGameInstance.ProcessChoice` _asbp_game_instance (`self.ButtonData`)))))

(event `ResetButton`
  (goto _label :!via `Reset`))

(fn `UserConstructionScript`
  (bind _aswbp_button_text (cast `/Game/UI/WBP_ButtonText` (`WidgetComponent.GetWidget` (`self.DescriptionWidget`))))
  (`TextBlock.SetText` (`/Game/UI/WBP_ButtonText.Txt_Description` _aswbp_button_text) (`KismetTextLibrary.Conv_StringToText` (`.Description` (break `ChoiceData` (`self.ButtonData`))))))